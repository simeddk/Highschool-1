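; BP_Player is a player character that moves sideways along world Y, jumps and makes sword-and-shield melee attacks, viewed through a camera set at BeginPlay.
; Left click plays a slash montage and sets IsAttacking, which blocks movement, jumping and re-attacking until EndAttack.
; OnCollision and OffCollision toggle a capsule hitbox that applies Atk damage to overlapped actors other than itself.
; Forward movement logic is disconnected.
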(event `self.ReceiveBeginPlay`
  ;[1 1 1] BeginPlay 카메라 세팅
  (`PlayerController.SetViewTargetWithBlend` (`GameplayStatics.GetPlayerController` 0) (`self.Camera`) 0.0 "VTBlend_Linear" 0.0 false)
  (`PrimitiveComponent.SetCollisionEnabled` (`self.Capsule`) "NoCollision"))

(event `InputAxis|MoveRight`
  (params (AxisValue :type "Float (single-precision)"))
  ;[1 1 1] 이동
  (if (not (`self.IsAttacking`))
    (`self.AddMovementInput` (0.0 1.0 0.0) AxisValue)))

(event `InputAxis|MoveForward`
  (params (AxisValue :type "Float (single-precision)"))
  ;[1 1 1] 이동
)

(event `Key|SpaceBar`
  (params (Key :type "Key Structure"))
  ;[1 1 1] 이동
  (:`Pressed`
    (if (not (`self.IsAttacking`))
      (`self.Jump`))))

(event `Key|LeftMouseButton`
  (params (Key :type "Key Structure"))
  ;[1 1 1] 공격
  (:`Pressed`
    (if (not (`self.IsAttacking`))
      (set `self.IsAttacking` true)
      (`self.PlayAnimMontage` "/Game/Mixamo/Paladin/Animations/sword_and_shield_slash_Montage.sword_and_shield_slash_Montage"))))

(event `EndAttack`
  ;[1 1 1] 공격
  (set `self.IsAttacking` false))

(event `self.Capsule.OnComponentBeginOverlap`
  (params (OverlappedComponent :type "PrimitiveComponent Object Reference") (OtherActor :type "Actor Object Reference") (OtherComp :type "PrimitiveComponent Object Reference") (OtherBodyIndex :type Integer) (bFromSweep :type Boolean) (SweepResult :type "HitResult Structure (by ref)"))
  (if (!= OtherActor self)
    (`GameplayStatics.ApplyDamage` OtherActor (`self.Atk`) null self)))

(event `OnCollision`
  (`PrimitiveComponent.SetCollisionEnabled` (`self.Capsule`) "QueryAndPhysics"))

(event `OffCollision`
  (`PrimitiveComponent.SetCollisionEnabled` (`self.Capsule`) "NoCollision"))

(fn `UserConstructionScript`)