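; BP_Mutant is a boss enemy that chases the player along the Y axis and attacks at close range.
; A Tick state machine drives approach and death cleanup, while StartAttack and EndAttack chain punches or a timer-charged skill with randomized threshold.
; Externally triggered events toggle punch and skill hitboxes that damage BP_Player.
; A dynamic material flashes on skills and hits, and death adds brief slow motion and camera shake.
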(event `self.ReceiveBeginPlay`
  ;[1 1 1] 비긴플레이 -> 다이나믹머티리얼 생성, 충돌체들 끄기
  (bind _returnvalue (`KismetMaterialLibrary.CreateDynamicMaterialInstance` "/Game/Mixamo/Mutant/mutant_M_Inst.mutant_M_Inst"))
  (bind _output_get (set `self.DynamicMaterial` _returnvalue))
  (`PrimitiveComponent.SetMaterial` (`self.Mesh`) 0 _output_get)
  (`PrimitiveComponent.SetCollisionEnabled` (`self.PunchCollision`) "NoCollision")
  (`PrimitiveComponent.SetCollisionEnabled` (`self.SkillCollision`) "NoCollision")
  (`KismetSystemLibrary.K2_SetTimerDelegate` (delegate `IncreaseSkillTime`) 1.0 true))

(event `IncreaseSkillTime`
  ;[1 1 1] 비긴플레이 -> 다이나믹머티리얼 생성, 충돌체들 끄기
  (`/Engine/EditorBlueprintResources/StandardMacros.IncrementFloat` (`self.SkillTime`)))

(event `self.ReceiveTick`
  (params (DeltaSeconds :type "Float (single-precision)"))
  (bind _returnvalue (- (`self.K2_GetActorLocation` (`GameplayStatics.GetPlayerCharacter` 0)) (`self.K2_GetActorLocation`)))
  (if (not (`self.IsPlayerDead`))
    (set `self.DistanceToPlayer` (`KismetMathLibrary.VSize` _returnvalue))
    (set `self.DirectionToPlayer` (`KismetMathLibrary.Normal` (`KismetMathLibrary.MakeVector` 0.0 (.y _returnvalue))))
    (switch `/Game/Enums/EStateType` (`self.State`)
      (:`NewEnumerator0`
        ;[1 1 1] Idle -> Approach
        (if (<= (`self.DistanceToPlayer`) 500.0)
          (set `self.State` "NewEnumerator1")))
      (:`NewEnumerator1`
        ;[1 1 1] Approach -> Attack
        (if (`self.IsAttacking`)
          _
          (elif (<= (`self.DistanceToPlayer`) 160.0)
            (`self.StartAttack`)
            (else
              (`self.AddMovementInput` (`self.DirectionToPlayer`))))))
      (:`NewEnumerator2`
        ;[1 1 1] Attack -> Approach
        (if (> (`self.DistanceToPlayer`) 180.0)
          (set `self.State` "NewEnumerator1")))
      (:`NewEnumerator3`
        ;[1 1 1] 5초후 시체 치우기
        (`KismetSystemLibrary.Delay` 5.0)
        (`self.K2_DestroyActor`)))))

(event `self.PunchCollision.OnComponentBeginOverlap`
  (params (OverlappedComponent :type "PrimitiveComponent Object Reference") (OtherActor :type "Actor Object Reference") (OtherComp :type "PrimitiveComponent Object Reference") (OtherBodyIndex :type Integer) (bFromSweep :type Boolean) (SweepResult :type "HitResult Structure (by ref)"))
  ;[1 1 1] 대미지 주기
  (if (!= OtherActor self)
    (if (== (`|GetArrayItem` (`ActorComponent.ComponentTags` OtherComp)) "Character")
      (bind _asbp_player (cast `/Game/Blueprints/BP_Player` OtherActor))
      (`GameplayStatics.ApplyDamage` _asbp_player (`self.Atk`) null self))))

(event `self.SkillCollision.OnComponentBeginOverlap`
  (params (OverlappedComponent :type "PrimitiveComponent Object Reference") (OtherActor :type "Actor Object Reference") (OtherComp :type "PrimitiveComponent Object Reference") (OtherBodyIndex :type Integer) (bFromSweep :type Boolean) (SweepResult :type "HitResult Structure (by ref)"))
  ;[1 1 1] 대미지 주기
  (if (!= OtherActor self)
    (if (== (`|GetArrayItem` (`ActorComponent.ComponentTags` OtherComp)) "Character")
      (bind _asbp_player (cast `/Game/Blueprints/BP_Player` OtherActor))
      (`GameplayStatics.ApplyDamage` _asbp_player (`self.SkillAtk`) null self))))

(event `OnCollision`
  ;[1 1 1] 충돌체 켜고 끄기
  (`PrimitiveComponent.SetCollisionEnabled` (`self.PunchCollision`) "QueryAndPhysics"))

(event `OnCollisionSkill`
  ;[1 1 1] 충돌체 켜고 끄기
  (`PrimitiveComponent.SetCollisionEnabled` (`self.SkillCollision`) "QueryAndPhysics"))

(event `OffCollision`
  ;[1 1 1] 충돌체 켜고 끄기
  (`PrimitiveComponent.SetCollisionEnabled` (`self.PunchCollision`) "NoCollision"))

(event `OffCollisionSkill`
  ;[1 1 1] 충돌체 켜고 끄기
  (`PrimitiveComponent.SetCollisionEnabled` (`self.SkillCollision`) "NoCollision"))

(event `StartAttack`
  ;[1 1 1] 공격 시작 전에 평타 혹은 스킬 몽타쥬 재생
  (`self.K2_SetActorRotation` (`KismetMathLibrary.Conv_VectorToRotator` (`self.DirectionToPlayer`)))
  (set `self.IsAttacking` true)
  (if (>= (`self.SkillTime`) (`KismetMathLibrary.RandomFloatInRange` 2.0 5.0))
    (set `self.State` "NewEnumerator4")
    (`MaterialInstanceDynamic.SetVectorParameterValue` (`self.DynamicMaterial`) "SkillColor" (struct :`B` 20.0 :`A` 1.0))
    (`self.PlayAnimMontage` "/Game/Mixamo/Mutant/Animations/Mutant_Flexing_Muscles_Montage.Mutant_Flexing_Muscles_Montage" 3.0 "Start")
    (`KismetSystemLibrary.Delay` 0.5)
    (`MaterialInstanceDynamic.SetVectorParameterValue` :`self` (`self.DynamicMaterial`) :`ParameterName` "SkillColor")
    (`self.PlayAnimMontage` "/Game/Mixamo/Mutant/Animations/Mutant_Swiping_Montage.Mutant_Swiping_Montage" 2.0 "None")
    (set `self.SkillTime` 0.0)
    (else
      (set `self.State` "NewEnumerator2")
      (`self.PlayAnimMontage` "/Game/Mixamo/Mutant/Animations/Zombie_Attack_Montage.Zombie_Attack_Montage" 1.2))))

(event `EndAttack`
  ;[1 1 1] 공격 끝난 후 다시 Approach 인지, 재공격할지
  (if (not (`self.IsPlayerDead`))
    (set `self.IsAttacking` false)
    (if (> (`self.DistanceToPlayer`) 160.0)
      (set `self.State` "NewEnumerator1")
      (else
        (`self.StartAttack`)))))

(event `self.ReceiveAnyDamage`
  (params (Damage :type "Float (single-precision)") (DamageType :type "DamageType Object Reference") (InstigatedBy :type "Controller Object Reference") (DamageCauser :type "Actor Object Reference"))
  ;[1 1 1] 대미지를 입었을 때
  (`self.ChangeHitColor`)
  (bind _output_get (set `self.HP` (- (`self.HP`) Damage)))
  (if (<= _output_get 0.0)
    (`GameplayStatics.SetGlobalTimeDilation` 0.25)
    (`PlayerCameraManager.PlayCameraShake` :`self` (`GameplayStatics.GetPlayerCameraManager` 0) :`ShakeClass` "/Game/Blueprints/BP_BossDying.BP_BossDying_C")
    (`self.PlayAnimMontage` "/Game/Mixamo/Mutant/Animations/Mutant_Dying_Montage.Mutant_Dying_Montage" 1.2 "Start")
    (set `self.State` "NewEnumerator3")
    (`PrimitiveComponent.SetCollisionEnabled` (`self.CapsuleComponent`) "NoCollision")
    (`PrimitiveComponent.SetCollisionEnabled` (`self.SkillCollision`) "NoCollision")
    (`PrimitiveComponent.SetCollisionEnabled` (`self.PunchCollision`) "NoCollision")
    (`KismetSystemLibrary.Delay` 0.2)
    (`GameplayStatics.SetGlobalTimeDilation` 1.0)))

(event `ChangeHitColor`
  ;[1 1 1] 대미지를 입었을 때
  (`MaterialInstanceDynamic.SetVectorParameterValue` (`self.DynamicMaterial`) "HitColor" (struct :`R` 1.0 :`A` 1.0))
  (`KismetSystemLibrary.Delay` 0.2)
  (`MaterialInstanceDynamic.SetVectorParameterValue` (`self.DynamicMaterial`) "HitColor" (struct :`A` 1.0)))

(fn `IsPlayerDead`
  (returns (IsDead :type Boolean))
  (bind _asbp_player (cast `/Game/Blueprints/BP_Player` (`GameplayStatics.GetPlayerCharacter` 0)))
  (return (`/Game/Blueprints/BP_Player.IsDead` _asbp_player)))

(fn `UserConstructionScript`)