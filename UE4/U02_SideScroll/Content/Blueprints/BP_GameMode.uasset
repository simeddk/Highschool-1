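; BP_GameMode is a game mode that tracks a boss character and puts up a stage-clear widget.
; On BeginPlay it finds the BP_Mutant tagged "Boss", then creates WB_StageClear and shows it immediately, independent of the boss's state.
; Tick polls the boss's State and, at one enum value, prints a Korean debug message announcing the boss's defeat every frame.
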(event `self.ReceiveBeginPlay`
  (bind _outactors (`GameplayStatics.GetAllActorsOfClass` "/Game/Blueprints/BP_Mutant.BP_Mutant_C"))
  (for _array_element _outactors
    (for _array_element_2 (`Actor.Tags` _array_element)
      (if (== _array_element_2 "Boss")
        (set `self.Boss` _array_element))))
  (bind _returnvalue (`|CreateWidget` "/Game/Widgets/WB_StageClear.WB_StageClear_C" (`GameplayStatics.GetPlayerController` 0)))
  (bind _output_get (set `self.StageClearWidget` _returnvalue))
  (`UserWidget.AddToViewport` _output_get 0)
  (`Widget.SetVisibility` (`self.StageClearWidget`) "Visible"))

(event `self.ReceiveTick`
  (params (DeltaSeconds :type "Float (single-precision)"))
  (bind _boss (`self.Boss`)
    (:`then`
      (if (`|EnumEquality` (`/Game/Blueprints/BP_Mutant.State` _boss) "NewEnumerator3")
        (`KismetSystemLibrary.PrintString` "보스의 목을 땄다.")))
    (:`else`)))

(fn `UserConstructionScript`)